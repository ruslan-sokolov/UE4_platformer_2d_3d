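; BP_interactiveBlock is a physics cube that the player ball can pull toward itself at the cost of energy.
; Overlapping its trigger enables input and shows a HUD prompt, while a physics constraint locks the cube's rotation.
; Holding Interact opens a Tick gate that drains player energy, updates a beam between ball and cube, and applies mass-scaled force toward the ball.
; Releasing Interact or running out of energy stops the pull.
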(event OnComponentBeginOverlap(DetectionTrigger)
  (params (OverlappedComponent :type Primitive%20Component%20Object%20Reference) (OtherActor :type Actor%20Object%20Reference) (OtherComp :type Primitive%20Component%20Object%20Reference) (OtherBodyIndex :type Integer) (bFromSweep :type Boolean) (SweepResult :type Hit%20Result%20Structure%20%28by%20ref%29))
  ;[1 1 1] Trigger Box
  (Utilities|FlowControl|Delay 0.3)
  (Utilities|Casting|CastToBP_PlayerBall OtherActor)
  (Input|EnableInput (Game|GetPlayerController 0))
  (Default|ShowInteractText (Variables|Default|GetUI_HUD)))

(event OnComponentEndOverlap(DetectionTrigger)
  (params (OverlappedComponent :type Primitive%20Component%20Object%20Reference) (OtherActor :type Actor%20Object%20Reference) (OtherComp :type Primitive%20Component%20Object%20Reference) (OtherBodyIndex :type Integer))
  ;[1 1 1] Trigger Box
  (Utilities|Casting|CastToBP_PlayerBall OtherActor)
  (Input|DisableInput (Game|GetPlayerController 0))
  (Default|HideInteractText (Variables|Default|GetUI_HUD)))

(event Custom|LockAllRotations
  (bind _physicsconstraint (Variables|Default|GetPhysicsConstraint))
  ;[1 1 1] Lock All Rotations
  (Class|PhysicsConstraintComponent|SetAngularSwing1Limit _physicsconstraint "ACM_Locked" 0.0)
  (Class|PhysicsConstraintComponent|SetAngularSwing2Limit _physicsconstraint "ACM_Locked" 0.0)
  (Class|PhysicsConstraintComponent|SetAngularTwistLimit _physicsconstraint "ACM_Locked" 0.0))

(event Custom|Close%20Interaction%20Gate
  (bind _player_ref (Variables|Default|GetPlayer_REF))
  (bind _staticmesh (Variables|Default|GetStaticMesh))
  (bind _player_ref_2 (Variables|Default|GetPlayer_REF))
  (bind _returnvalue (Transformation|GetActorLocation _player_ref_2))
  (bind _returnvalue_2 (Transformation|GetWorldLocation _staticmesh))
  (bind _returnvalue_3 (- _returnvalue _returnvalue_2))
  (Utilities|FlowControl|Sequence
    (:then_0
      (Components|Activation|Deactivate (Variables|Default|GetBeam))
      (Utilities|FlowControl|Gate true) ; enters at Close
    )
    (:then_1
      (Default|HideInteractText (Variables|Default|GetUI_HUD)))))

(event EventBeginPlay
  ;[1 1 1] Initialize The Cube
  (CallFunction|LockAllRotations)
  (Components|Activation|Deactivate (Variables|Default|GetBeam))
  (bind _asbp_player_ball (Utilities|Casting|CastToBP_PlayerBall (Game|Player|GetPlayerPawn 0)))
  (Utilities|FlowControl|Delay 0.2)
  (bind _output_get (Variables|Default|SetPlayer_REF _asbp_player_ball))
  (Variables|Default|SetUI_HUD (Variables|/Game/Blueprints/BP_PlayerBall.BP_PlayerBall_C|GetHUD_REF _output_get)))

(event EventTick
  (params (DeltaSeconds :type Float%20%28single-precision%29))
  (bind _player_ref (Variables|Default|GetPlayer_REF))
  (bind _staticmesh (Variables|Default|GetStaticMesh))
  (bind _player_ref_2 (Variables|Default|GetPlayer_REF))
  (bind _returnvalue (Transformation|GetActorLocation _player_ref_2))
  (bind _returnvalue_2 (Transformation|GetWorldLocation _staticmesh))
  (bind _returnvalue_3 (- _returnvalue _returnvalue_2))
  (Utilities|FlowControl|Gate true
    (:Exit
      (Utilities|IsValid (Variables|Default|GetPlayer_REF)
        (:Is%20Valid
          (Utilities|FlowControl|Sequence
            (:then_0
              ;[1 1 1] Drawn Player Energy
              (Default|EnergyDamage _player_ref 5e+01)
              (Class|ParticleSystemComponent|SetBeamSourcePoint (Variables|Default|GetBeam) 0 (Transformation|GetActorLocation _player_ref))
              (Class|ParticleSystemComponent|SetBeamTargetPoint (Variables|Default|GetBeam) 0 (Transformation|GetWorldLocation (Variables|Default|GetStaticMesh))))
            (:then_1
              ;[1 1 1] Pull Cube To The Ball
              (Math|Float|CompareFloat (Variables|/Game/Blueprints/BP_PlayerBall.BP_PlayerBall_C|GetEnergy (Variables|Default|GetPlayer_REF)) 0.5
                (:>
                  (Physics|AddForce _staticmesh (* (Math|Vector|Normalize (Math|Vector|MakeVector (.x _returnvalue_3) (.y _returnvalue_3) (.z _returnvalue_3))) (* (Physics|GetMass _staticmesh) 1e+03)) "None" false))
                (:==
                  (CallFunction|CloseInteractionGate :!label _label))
                (:<
                  (goto _label))))))))))

(event Input|ActionEvents|InputActionInteract
  (params (Key :type Key%20Structure :default "None"))
  (bind _player_ref (Variables|Default|GetPlayer_REF))
  (bind _staticmesh (Variables|Default|GetStaticMesh))
  (bind _player_ref_2 (Variables|Default|GetPlayer_REF))
  (bind _beam (Variables|Default|GetBeam))
  (bind _returnvalue (Transformation|GetActorLocation _player_ref_2))
  (bind _returnvalue_2 (Transformation|GetWorldLocation _staticmesh))
  (bind _returnvalue_3 (- _returnvalue _returnvalue_2))
  (:Pressed
    (Components|Activation|Activate _beam true)
    (Utilities|FlowControl|Gate true) ; enters at Open
  )
  (:Released
    (Components|Activation|Deactivate _beam)
    (Utilities|FlowControl|Gate true) ; enters at Close
  ))

(fn ConstructionScript)