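; BP_Elevator is a platform that the player ball raises by pressing Interact while inside its trigger.
; Entering the trigger enables input and shows the HUD interact prompt, while leaving hides it, disables input and sends the platform back down.
; Tick moves the actor vertically at SpeedOfPlatform, stopping once it reaches or passes UpLimit or DownLimit.
; The HUD reference comes from the player ball after a one-second delay on BeginPlay.
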(event OnComponentBeginOverlap(Trigger)
  (params (OverlappedComponent :type Primitive%20Component%20Object%20Reference) (OtherActor :type Actor%20Object%20Reference) (OtherComp :type Primitive%20Component%20Object%20Reference) (OtherBodyIndex :type Integer) (bFromSweep :type Boolean) (SweepResult :type Hit%20Result%20Structure%20%28by%20ref%29))
  ;[1 1 1] Trigger
  (Utilities|Casting|CastToBP_PlayerBall OtherActor)
  (Input|EnableInput (Game|GetPlayerController 0))
  (Default|ShowInteractText (Variables|Default|GetUI_HUD_REF)))

(event OnComponentEndOverlap(Trigger)
  (params (OverlappedComponent :type Primitive%20Component%20Object%20Reference) (OtherActor :type Actor%20Object%20Reference) (OtherComp :type Primitive%20Component%20Object%20Reference) (OtherBodyIndex :type Integer))
  ;[1 1 1] Trigger
  (Utilities|Casting|CastToBP_PlayerBall OtherActor)
  (Input|DisableInput (Game|GetPlayerController 0))
  (Default|HideInteractText (Variables|Default|GetUI_HUD_REF))
  (Variables|Default|SetIsMoving true)
  (Variables|Default|SetMoveUp false))

(event EventBeginPlay
  ;[1 1 1] Init
  (Utilities|FlowControl|Delay 1.0)
  (bind _asbp_player_ball (Utilities|Casting|CastToBP_PlayerBall (Game|GetPlayerCharacter 0)))
  (Variables|Default|SetUI_HUD_REF (Variables|/Game/Blueprints/BP_PlayerBall.BP_PlayerBall_C|GetHUD_REF _asbp_player_ball)))

(event EventTick
  (params (DeltaSeconds :type Float%20%28single-precision%29))
  (bind _returnvalue (Transformation|GetActorLocation))
  (bind _returnvalue_2 (Transformation|GetActorLocation))
  (bind _speedofplatform (Variables|Default|GetSpeedOfPlatform))
  (bind _speedofplatform_2 (Variables|Default|GetSpeedOfPlatform))
  (bind _returnvalue_3 (* _speedofplatform DeltaSeconds))
  (bind _returnvalue_4 (* _speedofplatform_2 DeltaSeconds))
  (bind _returnvalue_5 (- (.z _returnvalue_2) _returnvalue_4))
  (bind _returnvalue_6 (+ (.z _returnvalue) _returnvalue_3))
  (if (Variables|Default|GetIsMoving)
    (if (Variables|Default|GetMoveUp)
      (if (>= _returnvalue_6 (Variables|Default|GetUpLimit))
        (Variables|Default|SetIsMoving false))
      (Transformation|SetActorLocation (Math|Vector|MakeVector (.x _returnvalue) (.y _returnvalue) _returnvalue_6) false false)
      (else
        (if (<= _returnvalue_5 (Variables|Default|GetDownLimit))
          (Variables|Default|SetIsMoving false))
        (Transformation|SetActorLocation (Math|Vector|MakeVector (.x _returnvalue_2) (.y _returnvalue_2) _returnvalue_5) false false)))))

(event Input|ActionEvents|InputActionInteract
  (params (Key :type Key%20Structure :default "None"))
  ;[1 1 1] Interact
  (:Pressed
    (if (not (Variables|Default|GetIsMoving))
      (Variables|Default|SetMoveUp true)
      (Variables|Default|SetIsMoving true))))

(fn ConstructionScript)